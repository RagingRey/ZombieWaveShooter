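; Showcase variant of the West Patriot radar vehicle that exposes its configurable features to slider, checkbox and button controls.
; Sliders drive wheel speed, base rotation, radar elevation, holders, door angle and light emissivity, while a checkbox toggles damage and buttons pick the skin.
; Each indexed control event forwards straight to a setter defined outside this graph, and the construction script only calls the parent's.
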(event `self.SetSliderVariable0`
  (params (NewValue :type "Float (double-precision)"))
  ;[1 1 1] Showcase slider controls
  (`self.SetWheelSpeed` NewValue))

(event `self.SetCheckboxVariable0`
  (params (NewState :type Boolean))
  ;[1 1 1] Showcase checkbox controls
  (`self.SetShowDamaged` NewState))

(event `self.SetButtonsVariable0`
  (params (NewIndex :type Integer))
  ;[1 1 1] Showcase button controls
  (`self.SetSkinType` (`KismetMathLibrary.Conv_IntToDouble` NewIndex)))

(event `self.SetSliderVariable1`
  (params (NewValue :type "Float (double-precision)"))
  ;[1 1 1] Showcase slider controls
  (`self.SetBaseRotation` NewValue))

(event `self.SetSliderVariable2`
  (params (NewValue :type "Float (double-precision)"))
  ;[1 1 1] Showcase slider controls
  (`self.SetRadarElevation` NewValue))

(event `self.SetSliderVariable3`
  (params (NewValue :type "Float (double-precision)"))
  ;[1 1 1] Showcase slider controls
  (`self.SetHolders` NewValue))

(event `self.SetSliderVariable4`
  (params (NewValue :type "Float (double-precision)"))
  ;[1 1 1] Showcase slider controls
  (`self.SetDoorAngle` NewValue))

(event `self.SetSliderVariable5`
  (params (NewValue :type "Float (double-precision)"))
  ;[1 1 1] Showcase slider controls
  (`self.SetLightsEmissivity` NewValue))

(fn `UserConstructionScript`
  (`parent.UserConstructionScript`))