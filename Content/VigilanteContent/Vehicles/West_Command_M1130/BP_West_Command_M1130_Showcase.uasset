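; Showcase variant of the West Command M1130 vehicle that exposes its adjustable features to generic slider, checkbox and button controls.
; Numbered control events forward values to setters for motion, articulated parts, lights, skin, damaged-model visibility and firing.
; A twin slider drives mirror base and mirror rotation separately, and the skin button index converts to float.
; The construction script only runs the parent's version.
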(event `/Game/VigilanteContent/Shared/Blueprints/Showcase/Interfaces/BP_ShowcaseControlsInterface.SetSliderVariable0`
  (params (NewValue :type "Float (single-precision)"))
  ;[1 1 1] Speed
  (`self.SetWheelSpeed` NewValue))

(event `/Game/VigilanteContent/Shared/Blueprints/Showcase/Interfaces/BP_ShowcaseControlsInterface.SetButtonsVariable0`
  (params (NewIndex :type Integer))
  ;[1 1 1] Skin variant
  (`self.SetSkinType` (`KismetMathLibrary.Conv_IntToDouble` NewIndex)))

(event `/Game/VigilanteContent/Shared/Blueprints/Showcase/Interfaces/BP_ShowcaseControlsInterface.SetSliderVariable5`
  (params (NewValue :type "Float (single-precision)"))
  ;[1 1 1] Lights
  (`self.SetLightsEmissivity` NewValue))

(event `/Game/VigilanteContent/Shared/Blueprints/Showcase/Interfaces/BP_ShowcaseControlsInterface.SetSliderVariable1`
  (params (NewValue :type "Float (single-precision)"))
  ;[1 1 1] Wheel Angle
  (`self.SetWheelAngle` NewValue))

(event `/Game/VigilanteContent/Shared/Blueprints/Showcase/Interfaces/BP_ShowcaseControlsInterface.SetCheckboxVariable0`
  (params (NewState :type Boolean))
  ;[1 1 1] Damaged model visibility
  (`self.SetShowDamaged` NewState))

(event `/Game/VigilanteContent/Shared/Blueprints/Showcase/Interfaces/BP_ShowcaseControlsInterface.SetSliderVariable6`
  (params (NewValue :type "Float (single-precision)"))
  ;[1 1 1] Antenna Rotation
  (`self.SetAntennasAngle` NewValue))

(event `/Game/VigilanteContent/Shared/Blueprints/Showcase/Interfaces/BP_ShowcaseControlsInterface.SetSliderVariable2`
  (params (NewValue :type "Float (single-precision)"))
  ;[1 1 1] Turret rotation
  (`self.Set Turret Rotation` NewValue))

(event `/Game/VigilanteContent/Shared/Blueprints/Showcase/Interfaces/BP_ShowcaseControlsInterface.SetCheckboxVariable1`
  (params (NewState :type Boolean))
  ;[1 1 1] Firing activation
  (`self.SetFiringActive` NewState))

(event `/Game/VigilanteContent/Shared/Blueprints/Showcase/Interfaces/BP_ShowcaseControlsInterface.SetTwinSliderVariable0`
  (params (`bFirstSlider?` :type Boolean) (NewFirstValue :type "Float (single-precision)") (NewSecondValue :type "Float (single-precision)"))
  ;[1 1 1] Mirrors rotation
  (if `bFirstSlider?`
    (`self.SetMirrorsBaseRotation` NewFirstValue)
    (else
      (`self.SetMirrorsRotation` NewSecondValue))))

(event `/Game/VigilanteContent/Shared/Blueprints/Showcase/Interfaces/BP_ShowcaseControlsInterface.SetSliderVariable3`
  (params (NewValue :type "Float (single-precision)"))
  ;[1 1 1] Gun Elevation
  (`self.Set Gun Elevation` NewValue))

(event `/Game/VigilanteContent/Shared/Blueprints/Showcase/Interfaces/BP_ShowcaseControlsInterface.SetSliderVariable4`
  (params (NewValue :type "Float (single-precision)"))
  ;[1 1 1] Hatches
  (`self.SetHatchesRotation` NewValue))

(fn `UserConstructionScript`
  (`parent.UserConstructionScript`))